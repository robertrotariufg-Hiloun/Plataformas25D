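; BP_Enemy2 is a ranged enemy that periodically fires at the player when within range.
; A looping timer started on BeginPlay checks the distance to the Player reference, which is not assigned in these graphs.
; When in range, it spawns a Bullet at the Arrow1 component's world location and rotation, then plays the Cast montage.
; The graphs contain no aiming or movement logic, so shots follow the arrow's facing.
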(event Custom|DIsparar
  (if (< (Transformation|GetDistanceTo (Variables|Default|GetPlayer)) 1.5e+03)
    (Game|SpawnActorfromClass "/Game/Props/Bullet.Bullet_C" (Math|Transform|MakeTransform (Transformation|GetWorldLocation (Variables|Default|GetArrow1)) (Transformation|GetWorldRotation (Variables|Default|GetArrow1)) "1.000000,1.000000,1.000000") "Undefined" "MultiplyWithRoot" 0 0)
    (Animation|PlayAnimMontage "/Game/Enemy/AnimationsENmy2/Cast.Cast" 1.0 "None")))

(event EventBeginPlay
  (Utilities|Time|SetTimerbyEvent (delegate Custom|DIsparar) 2.0 true))

(event Collision|EventActorBeginOverlap
  (params (OtherActor :type Actor%20Object%20Reference)))

(event EventTick
  (params (DeltaSeconds :type Float%20%28single-precision%29)))

(fn ConstructionScript)
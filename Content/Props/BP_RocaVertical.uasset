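; BP_RocaVertical is a rock hazard prop that moves vertically and damages the player character, Prota, on contact.
; On BeginPlay it stores its start position and plays the MovimientoVertical timeline, offsetting Z by the curve value scaled by Altura.
; A Box overlap with Prota applies Damage once, guarded by PuedehacerDaño, then destroys the rock.
; The one-second flag reset follows DestroyActor, so the hit is effectively single-use.
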(event OnComponentBeginOverlap(Box)
  (params (OverlappedComponent :type Primitive%20Component%20Object%20Reference) (OtherActor :type Actor%20Object%20Reference) (OtherComp :type Primitive%20Component%20Object%20Reference) (OtherBodyIndex :type Integer) (bFromSweep :type Boolean) (SweepResult :type Hit%20Result%20Structure%20%28by%20ref%29))
  (bind _asprota (Utilities|Casting|CastToProta OtherActor))
  (if (Variables|Default|GetpuedehacerDaño)
    (Variables|Default|SetpuedehacerDaño false)
    (Default|TakeDamage _asprota (Variables|Default|GetDamage))
    (Actor|DestroyActor)
    (Utilities|FlowControl|Delay 1.0)
    (Variables|Default|SetpuedehacerDaño true)))

(event EventBeginPlay
  (Variables|Default|SetPosicionVertical (Transformation|GetActorLocation))
  (bind _newtrack_0 (Timeline|MovimientoVertical Play)
    (:Update
      (Transformation|SetActorLocation (+ (Math|Vector|MakeVector 0.0 0.0 (* _newtrack_0 (Variables|Default|Getaltura))) (Variables|Default|GetPosicionVertical)) false false))))

(event Collision|EventActorBeginOverlap
  (params (OtherActor :type Actor%20Object%20Reference)))

(event EventTick
  (params (DeltaSeconds :type Float%20%28single-precision%29)))

(fn ConstructionScript)